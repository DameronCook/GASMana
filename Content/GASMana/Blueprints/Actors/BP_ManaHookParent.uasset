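; BP_ManaHookParent is a grapple hook target actor whose look follows its GrappleType: ZipToPoint, Launch, LaunchUp or Swing.
; The construction script picks the matching mesh and scale, enlarging it for Swing.
; On BeginPlay it sets the matching brush on the WBP_HookImage in its TargetWidget component.
; SetActive passes false to the parent regardless of input, then shows or hides the target widget based on Active.
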(event EventBeginPlay
  (bind _aswbp_hook_image (Utilities|Casting|CastToWBP_HookImage (UserInterface|GetWidget (Variables|Default|GetTarget%20Widget))))
  (Class|Image|SetBrush (Variables|/Game/GASMana/UI/Widgets/HookTargets/WBP_HookImage.WBP_HookImage_C|GetTargetImage _aswbp_hook_image) (Class|WidgetBlueprintLibrary|MakeBrushfromAsset (Utilities|Select :Index (Variables|Default|GetGrappleType) :E_ZipToPoint "/Game/GASMana/UI/Textures/HookWidgetTextures/SlateBrush/SB_ZipToPointTarget.SB_ZipToPointTarget" :E_Launch "/Game/GASMana/UI/Textures/HookWidgetTextures/SlateBrush/SB_LaunchTarget.SB_LaunchTarget" :E_LaunchUp "/Game/GASMana/UI/Textures/HookWidgetTextures/SlateBrush/SB_LaunchUpTarget.SB_LaunchUpTarget" :E_Swing "/Game/GASMana/UI/Textures/HookWidgetTextures/SlateBrush/SB_SwingTarget.SB_SwingTarget"))))

(event EventSetActive
  (params (bActive :type Boolean))
  (Development|PrintString "HOLY SHIT I WAS CALLED" false false)
  (|CallParentFunction false)
  (bind _target_widget (Variables|Default|GetTarget%20Widget)
    (:then
      (Rendering|SetVisibility _target_widget bActive false))
    (:else)))

(fn ConstructionScript
  (Components|StaticMesh|SetStaticMesh (Variables|Character|GetMesh) (Utilities|Select :Index (Variables|Default|GetGrappleType) :E_ZipToPoint (Variables|Default|GetZipToPointMesh) :E_Launch (Variables|Default|GetLaunchMesh) :E_LaunchUp (Variables|Default|GetLaunchUpMesh) :E_Swing (Variables|Default|GetSwingMesh)))
  (Transformation|SetRelativeScale3D (Variables|Character|GetMesh) (Utilities|Select :Index (Variables|Default|GetGrappleType) :E_ZipToPoint "1.000000,1.000000,1.000000" :E_Launch "1.000000,1.000000,1.000000" :E_LaunchUp "1.000000,1.000000,1.000000" :E_Swing "3.000000,3.000000,3.000000")))