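; Base grapple hook point actor that shows a target indicator for one of four grapple types: zip-to-point, launch, launch-up or swing.
; The construction script picks mesh and scale from GrappleType, and BeginPlay sets the matching widget icon.
; SetActive toggles the widget and plays its activation animation once, which ends enlarged and white.
; Reset, or Tick while the widget is hidden, stops the animation and restores the small grey look.
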(event Custom|Set%20Size
  (bind _target_widget (Variables|Default|GetTarget%20Widget))
  (bind _returnvalue (UserInterface|GetWidget _target_widget))
  (bind _aswbp_hook_image (Utilities|Casting|CastToWBP_HookImage _returnvalue))
  (Class|UserWidget|StopAnimation _returnvalue (Variables|/Game/GASMana/UI/Widgets/HookTargets/WBP_HookImage.WBP_HookImage_C|GetActivated _aswbp_hook_image))
  (Widget|Transform|SetRenderScale (Variables|/Game/GASMana/UI/Widgets/HookTargets/WBP_HookImage.WBP_HookImage_C|GetTargetImage _aswbp_hook_image) "(X=1.500000,Y=1.500000)")
  (Appearance|SetColorandOpacity (Variables|/Game/GASMana/UI/Widgets/HookTargets/WBP_HookImage.WBP_HookImage_C|GetTargetImage _aswbp_hook_image) "(R=1.000000,G=1.000000,B=1.000000,A=1.000000)" :!class /Script/UMG.Image))

(event Custom|Reset
  (bind _target_widget (Variables|Default|GetTarget%20Widget))
  (bind _returnvalue (UserInterface|GetWidget _target_widget))
  (Variables|Default|SetbAnimationPlayed false)
  (bind _aswbp_hook_image (Utilities|Casting|CastToWBP_HookImage _returnvalue))
  (Class|UserWidget|StopAnimation _returnvalue (Variables|/Game/GASMana/UI/Widgets/HookTargets/WBP_HookImage.WBP_HookImage_C|GetActivated _aswbp_hook_image))
  (Widget|Transform|SetRenderScale (Variables|/Game/GASMana/UI/Widgets/HookTargets/WBP_HookImage.WBP_HookImage_C|GetTargetImage _aswbp_hook_image) "(X=1.000000,Y=1.000000)")
  (Appearance|SetColorandOpacity (Variables|/Game/GASMana/UI/Widgets/HookTargets/WBP_HookImage.WBP_HookImage_C|GetTargetImage _aswbp_hook_image) "(R=0.500000,G=0.500000,B=0.500000,A=1.000000)" :!class /Script/UMG.Image))

(event EventBeginPlay
  (bind _target_widget (Variables|Default|GetTarget%20Widget))
  (bind _returnvalue (UserInterface|GetWidget _target_widget))
  (bind _aswbp_hook_image (Utilities|Casting|CastToWBP_HookImage _returnvalue))
  (Class|Image|SetBrush (Variables|/Game/GASMana/UI/Widgets/HookTargets/WBP_HookImage.WBP_HookImage_C|GetTargetImage _aswbp_hook_image) (Class|WidgetBlueprintLibrary|MakeBrushfromAsset (Utilities|Select :Index (Variables|Default|GetGrappleType) :E_ZipToPoint "/Game/GASMana/UI/Textures/HookWidgetTextures/SlateBrush/SB_ZipToPointTarget.SB_ZipToPointTarget" :E_Launch "/Game/GASMana/UI/Textures/HookWidgetTextures/SlateBrush/SB_LaunchTarget.SB_LaunchTarget" :E_LaunchUp "/Game/GASMana/UI/Textures/HookWidgetTextures/SlateBrush/SB_LaunchUpTarget.SB_LaunchUpTarget" :E_Swing "/Game/GASMana/UI/Textures/HookWidgetTextures/SlateBrush/SB_SwingTarget.SB_SwingTarget")))
  (Class|UserWidget|BindtoAnimationFinished _returnvalue (Variables|/Game/GASMana/UI/Widgets/HookTargets/WBP_HookImage.WBP_HookImage_C|GetActivated _aswbp_hook_image) (delegate Custom|Set%20Size)))

(event EventTick
  (params (DeltaSeconds :type Float%20%28single-precision%29))
  (bind _target_widget (Variables|Default|GetTarget%20Widget))
  (bind _returnvalue (UserInterface|GetWidget _target_widget))
  (if (not (Rendering|IsVisible (Variables|Default|GetTarget%20Widget)))
    (Variables|Default|SetbAnimationPlayed false)
    (bind _aswbp_hook_image (Utilities|Casting|CastToWBP_HookImage _returnvalue))
    (Class|UserWidget|StopAnimation _returnvalue (Variables|/Game/GASMana/UI/Widgets/HookTargets/WBP_HookImage.WBP_HookImage_C|GetActivated _aswbp_hook_image))
    (Widget|Transform|SetRenderScale (Variables|/Game/GASMana/UI/Widgets/HookTargets/WBP_HookImage.WBP_HookImage_C|GetTargetImage _aswbp_hook_image) "(X=1.000000,Y=1.000000)")
    (Appearance|SetColorandOpacity (Variables|/Game/GASMana/UI/Widgets/HookTargets/WBP_HookImage.WBP_HookImage_C|GetTargetImage _aswbp_hook_image) "(R=0.500000,G=0.500000,B=0.500000,A=1.000000)" :!class /Script/UMG.Image)))

(event EventSetActive
  (params (bActive :type Boolean))
  (|CallParentFunction bActive)
  (bind _target_widget (Variables|Default|GetTarget%20Widget)
    (:then
      (Rendering|SetVisibility _target_widget bActive false)
      (if (and bActive (not (Variables|Default|GetbAnimationPlayed)))
        (Variables|Default|SetbAnimationPlayed true)
        (bind _aswbp_hook_image (Utilities|Casting|CastToWBP_HookImage (UserInterface|GetWidget _target_widget)))
        (UserInterface|Animation|PlayAnimation (UserInterface|GetWidget _target_widget) (Variables|/Game/GASMana/UI/Widgets/HookTargets/WBP_HookImage.WBP_HookImage_C|GetActivated _aswbp_hook_image) 0.0 1 "Forward" 1.0 false)))
    (:else)))

(fn ConstructionScript
  (Components|StaticMesh|SetStaticMesh (Variables|Character|GetMesh) (Utilities|Select :Index (Variables|Default|GetGrappleType) :E_ZipToPoint (Variables|Default|GetZipToPointMesh) :E_Launch (Variables|Default|GetLaunchMesh) :E_LaunchUp (Variables|Default|GetLaunchUpMesh) :E_Swing (Variables|Default|GetSwingMesh)))
  (Transformation|SetRelativeScale3D (Variables|Character|GetMesh) (Utilities|Select :Index (Variables|Default|GetGrappleType) :E_ZipToPoint "1.000000,1.000000,1.000000" :E_Launch "1.000000,1.000000,1.000000" :E_LaunchUp "1.000000,1.000000,1.000000" :E_Swing "3.000000,3.000000,3.000000")))

(fn BPManaHookParentAutoGenFunc
  (params (InVisibility :type ESlateVisibility%20Enum :default "Visible")))