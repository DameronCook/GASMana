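; BP_LorePopUp is a trigger-box actor that lets the player investigate a piece of lore.
; When BP_PlayerManaCharacter enters the box, it shows the character's Investigate widget and enables CanInvestigate.
; It also reads Title and Lore from its configured data table row and passes them to the character's Lore widget.
; Leaving the box removes the prompt and disables investigation.
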(event OnComponentBeginOverlap(Box)
  (params (OverlappedComponent :type Primitive%20Component%20Object%20Reference) (OtherActor :type Actor%20Object%20Reference) (OtherComp :type Primitive%20Component%20Object%20Reference) (OtherBodyIndex :type Integer) (bFromSweep :type Boolean) (SweepResult :type Hit%20Result%20Structure%20%28by%20ref%29))
  (bind _datatable (Variables|Default|GetDataTable))
  (bind (_datatable_2 _rowname) (Utilities|Struct|BreakDataTableRowHandle _datatable))
  (bind _asbp_player_mana_character (Utilities|Casting|CastToBP_PlayerManaCharacter OtherActor))
  (Development|PrintString "Set Lore")
  (UserInterface|Viewport|AddtoViewport (Variables|/Game/GASMana/Blueprints/Actors/BP_PlayerManaCharacter.BP_PlayerManaCharacter_C|GetInvestigate%20Widget _asbp_player_mana_character) 0)
  (Variables|/Game/GASMana/Blueprints/Actors/BP_PlayerManaCharacter.BP_PlayerManaCharacter_C|SetCanInvestigate _asbp_player_mana_character true)
  (bind _returnvalue (Utilities|GetDataTableRow _datatable_2 _rowname)
    (:then
      (Default|SetLore (Variables|/Game/GASMana/Blueprints/Actors/BP_PlayerManaCharacter.BP_PlayerManaCharacter_C|GetLoreWidget _asbp_player_mana_character) (.Title (Utilities|Struct|BreakST_LorePopUpData _returnvalue)) (.Lore (Utilities|Struct|BreakST_LorePopUpData _returnvalue))))))

(event OnComponentEndOverlap(Box)
  (params (OverlappedComponent :type Primitive%20Component%20Object%20Reference) (OtherActor :type Actor%20Object%20Reference) (OtherComp :type Primitive%20Component%20Object%20Reference) (OtherBodyIndex :type Integer))
  (bind _asbp_player_mana_character (Utilities|Casting|CastToBP_PlayerManaCharacter OtherActor))
  (Widget|RemovefromParent (Variables|/Game/GASMana/Blueprints/Actors/BP_PlayerManaCharacter.BP_PlayerManaCharacter_C|GetInvestigate%20Widget _asbp_player_mana_character))
  (Variables|/Game/GASMana/Blueprints/Actors/BP_PlayerManaCharacter.BP_PlayerManaCharacter_C|SetCanInvestigate _asbp_player_mana_character false))

(event Custom|SetLore)

(event EventBeginPlay)

(fn ConstructionScript)